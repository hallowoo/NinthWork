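; BP_WNController is the player controller that relays chat and match events between the WBP_ChatUI widget and BP_WNGameModeBase in a networked turn-based game.
; On BeginPlay it shows the cursor, finds the chat widget after a short delay and binds its message event.
; It forwards messages, user IDs and readiness to the game mode.
; It pushes broadcasts, user list, ID confirmation, scores, turn colors and timer updates to the widget.
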(event `self.ReceiveBeginPlay`
  ; Initialize & Capture Massages
  (set `self.bShowMouseCursor` true)
  (if (not (`|EnumEquality` (`self.GetRemoteRole`) "ROLE_None"))
    (`KismetSystemLibrary.Delay` 0.1)
    (bind _foundwidgets (`WidgetBlueprintLibrary.GetAllWidgetsOfClass` "/Game/Bluprints/Widget/WBP_ChatUI.WBP_ChatUI_C"))
    (bind _output_get (set `self.Widget` (`|GetArrayItem` _foundwidgets)))
    (bind _aswbp_chat_ui (cast `/Game/Bluprints/Widget/WBP_ChatUI` _output_get))
    (bind _output_get_2 (set `self.As WBP Chat UI` _aswbp_chat_ui))
    (add `/Game/Bluprints/Widget/WBP_ChatUI.SetUserMassage` _output_get_2 (`|CreateDelegate` :!event `SendMassageToServer`))))

(event `SendMassageToServer`
  (params (Massage :type String))
  ; To Server
  ;; Send Massage To Server
  (bind _asbp_wngame_mode_base (cast `/Game/Bluprints/Core/BP_WNGameModeBase` (`GameplayStatics.GetGameMode`)))
  (`/Game/Bluprints/Core/BP_WNGameModeBase.MassageFromUser` _asbp_wngame_mode_base Massage self))

(event `GotBroadcast`
  (params (Massage :type String) (TextColor :type "LinearColor Structure"))
  ; To UI
  ;; Massage To UI From GameMode
  (`/Engine/EditorBlueprintResources/StandardMacros.IsValid` (`self.As WBP Chat UI`)
    (:`Is Valid`
      (`/Game/Bluprints/Widget/WBP_ChatUI.AddChatToChatWindow` (`self.As WBP Chat UI`) Massage TextColor))
    (:`Is Not Valid`
      (`KismetSystemLibrary.Delay` 0.5)
      (`/Game/Bluprints/Widget/WBP_ChatUI.AddChatToChatWindow` (`self.As WBP Chat UI`) Massage TextColor))))

(event `SetIDToState`
  (params (ID :type String))
  ; To Server
  ;; Send ID by User To State From User
  (bind _asbp_wngame_mode_base (cast `/Game/Bluprints/Core/BP_WNGameModeBase` (`GameplayStatics.GetGameMode`)))
  (`/Game/Bluprints/Core/BP_WNGameModeBase.SendIDToState` _asbp_wngame_mode_base ID self))

(event `SetWhoIsThis`
  (params (Who :type String))
  ; To UI
  ;; Send Authority Info To UI
  (`self.SendWhoInfo` Who))

(event `AddIDToUI`
  (params (UserID :type String))
  ; To UI
  ;; Send ID by User To UI From State
  (`/Game/Bluprints/Widget/WBP_ChatUI.AddUserIDToUserList` (`self.As WBP Chat UI`) UserID))

(event `ScoreUIUpdate`
  (params (WinnerID :type String) (Score :type Integer))
  ; To UI
  ;; ScoreUI Update
  (`/Game/Bluprints/Widget/WBP_ChatUI.UpdateScoreUI` (`self.As WBP Chat UI`) WinnerID Score))

(event `IDConfirm`
  ; To UI
  ;; ID Confirm
  (`/Game/Bluprints/Widget/WBP_ChatUI.IDIsConfirmed` (`self.As WBP Chat UI`)))

(event `GameReady`
  ; To Server
  ;; Notify Ready To Game
  (bind _asbp_wngame_mode_base (cast `/Game/Bluprints/Core/BP_WNGameModeBase` (`GameplayStatics.GetGameMode`)))
  (`/Game/Bluprints/Core/BP_WNGameModeBase.GameIsReady` _asbp_wngame_mode_base self))

(event `ChangeScoreTextColor`
  (params (PlayerIndex :type Integer) (TextColor :type "LinearColor Structure"))
  ; To UI
  ;; Change Scoreboard Color On Turn
  (`/Game/Bluprints/Widget/WBP_ChatUI.ChangeScoreColor` (`self.As WBP Chat UI`) PlayerIndex TextColor))

(event `SendRemainingTimeToUI`
  (params (Time :type "Float (double-precision)"))
  ; To UI
  ;; Update Remaining Time
  (`/Game/Bluprints/Widget/WBP_ChatUI.UpdateTimer` (`self.As WBP Chat UI`) Time))

(fn `UserConstructionScript`)