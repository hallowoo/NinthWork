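; BP_WNPlayerState is the player state handling a player's ID registration, turns, score, out status and reset.
; SetID checks length and uniqueness against the game state's PlayerList, then registers and confirms the player or reports errors through the game mode.
; New IDs and win scores reach the UI by looping over every BP_WNController.
; Turn, out and reset events simply wrap functions defined outside these graphs.
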(event `SetID`
  (params (ID :type String))
  (bind _returnvalue (`KismetStringLibrary.Len` ID))
  (bind _registeredid (`self.RegisteredID`))
  ; Set ID
  (bind _asbp_wngame_mode_base (cast `/Game/Bluprints/Core/BP_WNGameModeBase` (`GameplayStatics.GetGameMode`)))
  (bind _asbp_wncontroller (cast `/Game/Bluprints/Core/BP_WNController` (`self.GetOwner`)))
  (if (> _returnvalue 10)
    (`/Game/Bluprints/Core/BP_WNGameModeBase.PlayerGetSystemMassage` _asbp_wngame_mode_base "Please enter ID with 10 characters or less." _asbp_wncontroller)
    (elif (> 1 _returnvalue)
      (`/Game/Bluprints/Core/BP_WNGameModeBase.PlayerGetSystemMassage` _asbp_wngame_mode_base "Please enter at least one character for your ID." _asbp_wncontroller)
      (else
        (bind _asbp_wngame_state_base (cast `/Game/Bluprints/Core/BP_WNGameStateBase` (`GameplayStatics.GetGameState`)))
        (for _array_element (`/Game/Bluprints/Core/BP_WNGameStateBase.PlayerList` _asbp_wngame_state_base)
          (bind _asbp_wnplayer_state (cast `/Game/Bluprints/Core/BP_WNPlayerState` (`Controller.PlayerState` _array_element)))
          (`KismetArrayLibrary.Array_Add` _registeredid (`WNPlayerState.UserID` _asbp_wnplayer_state)))
        (if (== -1 (`KismetArrayLibrary.Array_Find` _registeredid ID))
          (`self.SetUserID` ID)
          (`self.SendUserInfoToCreateUI`)
          (`/Game/Bluprints/Core/BP_WNGameStateBase.PlayerRegistration` _asbp_wngame_state_base _asbp_wncontroller)
          (`/Game/Bluprints/Core/BP_WNController.IDConfirm` _asbp_wncontroller)
          (else
            (`/Game/Bluprints/Core/BP_WNGameModeBase.PlayerGetSystemMassage` _asbp_wngame_mode_base "This ID is already exist." _asbp_wncontroller)))))))

(event `SendUserInfoToCreateUI`
  ; To Create ID UI
  (bind _outactors (`GameplayStatics.GetAllActorsOfClass` "/Game/Bluprints/Core/BP_WNController.BP_WNController_C"))
  (for _array_element _outactors
    (`/Game/Bluprints/Core/BP_WNController.AddIDToUI` _array_element (`self.GetUserID`))))

(event `SpendTurn`
  ; Use Turn
  (`self.PlayerUseTurn`))

(event `PlayerWin`
  (params (WinnerID :type String))
  ; Player Win
  (`self.PlayerGetScore`)
  (`self.SendNewScore` WinnerID))

(event `SendNewScore`
  (params (WinnerID :type String))
  ; Scoreboard Update
  (bind _outactors (`GameplayStatics.GetAllActorsOfClass` "/Game/Bluprints/Core/BP_WNController.BP_WNController_C"))
  (for _array_element _outactors
    (`/Game/Bluprints/Core/BP_WNController.ScoreUIUpdate` _array_element WinnerID (`self.PlayerScore`))))

(event `PlayerIsOut`
  ; Player Out
  (`self.PlayerOut`))

(event `ResetPlayerState`
  ; Reset State
  (`self.InitializeState`))

(fn `UserConstructionScript`)