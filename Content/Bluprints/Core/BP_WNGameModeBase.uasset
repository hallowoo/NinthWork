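; Game mode for a multiplayer chat-based Bulls and Cows number guessing game, with host-started rounds, turns and win/out handling.
; Chat input is routed to commands ('!play'), slash-prefixed guesses scored as strikes and balls, or plain chat.
; Turns rotate through the GameState player list on a timer, skipping out players.
; Messages, countdown and scoreboard colors are pushed to every BP_WNController, alongside sound cues.
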(event `WelcomMassage`
  (params (PlayerController :type "/Game/Bluprints/Core/BP_WNController Object Reference"))
  ; WelcomeMassage
  (`/Game/Bluprints/Core/BP_WNController.GotBroadcast` PlayerController "Welcome to Bulls and Cows!" (struct :`B` 0.75 :`A` 1.0))
  (`/Game/Bluprints/Core/BP_WNController.GotBroadcast` PlayerController "Please enter your ID first." (struct :`G` 0.5 :`A` 1.0))
  (if (`Controller.IsLocalController` PlayerController)
    (`KismetSystemLibrary.Delay` 0.5)
    (`self.PlaySound` "Crowd")
    (`self.PlaySound` "Opening")))

(event `MassageFromUser`
  (params (Massage :type String) (PlayerController :type "/Game/Bluprints/Core/BP_WNController Object Reference"))
  (bind _currentplayercontroller (`self.CurrentPlayerController`))
  (bind _bp_wngame_state_base (`self.BP WNGame State Base`))
  ; Chat & Answer
  ;; Massage From User
  (if (`KismetStringLibrary.IsEmpty` Massage)
    (`self.PlayerGetSystemMassage` "Please enter at least one character" PlayerController)
    (else
      (bind _asbp_wngame_state_base (cast `/Game/Bluprints/Core/BP_WNGameStateBase` (`GameplayStatics.GetGameState`)))
      (bind _output_get (set `self.BP WNGame State Base` _asbp_wngame_state_base))
      (if (== (`KismetArrayLibrary.Array_Find` (`/Game/Bluprints/Core/BP_WNGameStateBase.PlayerList` _output_get) PlayerController) -1)
        (`self.PlayerGetSystemMassage` "Please Enter Your ID." PlayerController)
        (else
          (set `self.CurrentPlayerController` PlayerController)
          (bind _asbp_wnplayer_state (cast `/Game/Bluprints/Core/BP_WNPlayerState` (`Controller.PlayerState` (`self.CurrentPlayerController`))))
          (bind _output_get_2 (set `self.BP WNPlayer State` _asbp_wnplayer_state))
          (`/Game/Bluprints/Core/BP_WNGameStateBase.SaveChatList` (`self.BP WNGame State Base`) (`KismetStringLibrary.Concat_StrStr` (`WNPlayerState.UserID` _output_get_2) " : " Massage))
          (bind _returnvalue (`IdentifyingCommands.IsCommand` Massage))
          (if _returnvalue
            (`self.GetCommand` Massage)
            (elif (`KismetStringLibrary.EqualEqual_StrStr` (`KismetStringLibrary.GetSubstring` Massage) "/")
              (if (`/Game/Bluprints/Core/BP_WNGameStateBase.IsGameInPlay` (`self.BP WNGame State Base`))
                (if (`WNPlayerState.bHasTicket` (`self.BP WNPlayer State`))
                  (if (`WNPlayerState.bIsOut` (`self.BP WNPlayer State`))
                    (`self.PlayerGetSystemMassage` "You used all chances." (`self.CurrentPlayerController`))
                    (elif (== (`/Game/Bluprints/Core/BP_WNGameStateBase.TurnIndex` _bp_wngame_state_base) (`KismetArrayLibrary.Array_Find` (`/Game/Bluprints/Core/BP_WNGameStateBase.PlayerList` _bp_wngame_state_base) (`self.CurrentPlayerController`)))
                      (bind _returnvalue_2 (`AnswerOrNot.AnswerOrNot` Massage))
                      (if _returnvalue_2
                        (if (> (`WNPlayerState.GetRemainingTurn` (`self.BP WNPlayer State`)) 0)
                          (`self.AnswerDecision` Massage)
                          (else
                            (`self.PlayerGetSystemMassage` "You used all chances" (`self.CurrentPlayerController`))))
                        (else
                          (`self.SendBroadcast` (`KismetStringLibrary.Concat_StrStr` Massage " is Incorrect answer format") (`self.AnswerTextColor`))
                          (`/Game/Bluprints/Core/BP_WNPlayerState.SpendTurn` (`self.BP WNPlayer State`))
                          (`self.BroadcastRemainingTurn`)
                          (`self.OutDecision` (`self.CurrentPlayerController`))))
                      (else
                        (`self.PlayerGetSystemMassage` "Please wait until your turn" (`self.CurrentPlayerController`)))))
                  (else
                    (`self.PlayerGetSystemMassage` "Please join the next game" (`self.CurrentPlayerController`))))
                (else
                  (`self.PlayerGetSystemMassage` "Game is not in play." _currentplayercontroller)
                  (`self.PlayerGetSystemMassage` "If you want to play the game, enter '!play' on host" _currentplayercontroller)))
              (else
                (`self.SendBroadcast` (`KismetStringLibrary.Concat_StrStr` (`WNPlayerState.UserID` (`self.BP WNPlayer State`)) " : " Massage) (`self.DefaultTextColor`))))))))))

(event `AnswerDecision`
  (params (Massage :type String))
  (bind _bp_wnplayer_state (`self.BP WNPlayer State`))
  (bind _bp_wnplayer_state_2 (`self.BP WNPlayer State`))
  (bind _userid (`WNPlayerState.UserID` _bp_wnplayer_state_2))
  ; Chat & Answer
  ;; Answer Decision And Post Processing
  (`|ExecutionSequence`
    (:`then_0`
      (bind _returnvalue (`StrikeOrBall.StrikeOrBall` Massage (`WNGameStateBase.GetGoalNumber` (`self.BP WNGame State Base`))))
      (set `self.StrikeCount` (break `IntPoint` _returnvalue))
      (set `self.BallCount` (`.Y` (break `IntPoint` _returnvalue)))
      (bind _asbp_wnplayer_state (cast `/Game/Bluprints/Core/BP_WNPlayerState` (`Controller.PlayerState` (`self.CurrentPlayerController`))))
      (set `self.BP WNPlayer State` _asbp_wnplayer_state)
      (`/Game/Bluprints/Core/BP_WNPlayerState.SpendTurn` _bp_wnplayer_state)
      (`self.SendBroadcast` (`KismetStringLibrary.Concat_StrStr` (`KismetStringLibrary.Concat_StrStr` (`WNPlayerState.UserID` _bp_wnplayer_state) " : " Massage " is ") (`KismetStringLibrary.Conv_IntToString` (`self.StrikeCount`)) "S" (`KismetStringLibrary.Conv_IntToString` (`self.BallCount`)) "B") (`self.AnswerTextColor`)))
    (:`then_1`
      (bind _returnvalue_2 (`AnswerIsCorrect.AnswerIsCorrect` (`self.StrikeCount`)))
      (if _returnvalue_2
        (`self.StopTimer`)
        (`/Game/Bluprints/Core/BP_WNPlayerState.PlayerWin` _bp_wnplayer_state_2 _userid)
        (`self.StopSound` "Background")
        (`self.PlaySound` "BatHit")
        (`self.PlaySound` "Homerun")
        (`self.PlaySound` "HomerunSong")
        (`self.SendBroadcast` (`KismetStringLibrary.Concat_StrStr` "Homerun!!" _userid " is win! Get score +1!") (`self.DefaultTextColor`))
        (`self.GameOver`)
        (else
          (`self.BroadcastRemainingTurn`)
          (`self.OutDecision` (`self.CurrentPlayerController`)))))))

(event `GetCommand`
  (params (Command :type String))
  (bind _currentplayercontroller (`self.CurrentPlayerController`))
  ; Chat & Answer
  ;; Get Command
  (switch `string` Command
    (:`Default`
      (`self.PlayerGetSystemMassage` "Incorrect command" _currentplayercontroller))
    (:`!play`
      (bind _asbp_wngame_state_base (cast `/Game/Bluprints/Core/BP_WNGameStateBase` (`GameplayStatics.GetGameState`)))
      (if (`/Game/Bluprints/Core/BP_WNGameStateBase.IsGameInPlay` _asbp_wngame_state_base)
        (`self.PlayerGetSystemMassage` "Can't start new game in play" _currentplayercontroller)
        (else
          (`self.StopSound` "AllSound")
          (if (`Controller.IsLocalController` (`self.CurrentPlayerController`))
            (`self.ResetGame`)
            (`self.TicketToUser`)
            (`self.GameStart`)
            (`self.SendBroadcast` "Host start game! Let's play!" (`self.DefaultTextColor`))
            (`self.PlaySound` "Background")
            (bind _asbp_wnplayer_state (cast `/Game/Bluprints/Core/BP_WNPlayerState` (`Controller.PlayerState` (`|GetArrayItem` (`/Game/Bluprints/Core/BP_WNGameStateBase.PlayerList` (`self.BP WNGame State Base`))))))
            (`self.SendBroadcast` (`KismetStringLibrary.Concat_StrStr` (`WNPlayerState.UserID` _asbp_wnplayer_state) "'s turn.") (struct :`R` 1.0 :`G` 0.502887 :`A` 1.0))
            (`self.ChangeScoreColorOnTurn` 0 (`self.ScoreColorOnTurn`))
            (`self.StartTimer`)
            (else
              (`self.PlayerGetSystemMassage` "Only the host can start play" _currentplayercontroller))))))))

(event `PlayerGetSystemMassage`
  (params (Massage :type String) (PlayerController :type "/Game/Bluprints/Core/BP_WNController Object Reference"))
  ; Chat To User
  ;; Private System Massage
  (`/Engine/EditorBlueprintResources/StandardMacros.IsValid` PlayerController
    (:`Is Valid`
      (`/Game/Bluprints/Core/BP_WNController.GotBroadcast` PlayerController Massage (struct :`G` 0.5 :`A` 1.0)))))

(event `SendBroadcast`
  (params (Massage :type String) (TextColor :type "LinearColor Structure"))
  ; Chat To User
  ;; Global Chat
  (bind _outactors (`GameplayStatics.GetAllActorsOfClass` "/Game/Bluprints/Core/BP_WNController.BP_WNController_C"))
  (for _array_element _outactors
    (`/Game/Bluprints/Core/BP_WNController.GotBroadcast` _array_element Massage TextColor)))

(event `ResetGame`
  ; Game & Player State
  ;; Reset Game
  (bind _outactors (`GameplayStatics.GetAllActorsOfClass` "/Game/Bluprints/Core/BP_WNController.BP_WNController_C"))
  (for _array_element _outactors
    (bind _asbp_wnplayer_state (cast `/Game/Bluprints/Core/BP_WNPlayerState` (`Controller.PlayerState` _array_element)))
    (`/Game/Bluprints/Core/BP_WNPlayerState.ResetPlayerState` _asbp_wnplayer_state)
    (bind _asbp_wngame_state_base (cast `/Game/Bluprints/Core/BP_WNGameStateBase` (`GameplayStatics.GetGameState`)))
    (`/Game/Bluprints/Core/BP_WNGameStateBase.ResetGameState` _asbp_wngame_state_base)))

(event `PlaySound`
  (params (SoundName :type String))
  ; Sounds
  ;; PlaySound
  (switch `string` SoundName
    (:`Crowd`
      (`AudioComponent.Play` (`self.SQ_Crowd`) 0.0))
    (:`Opening`
      (`AudioComponent.Play` (`self.SQ_Opening`) 0.0))
    (:`Background`
      (`AudioComponent.Play` (`self.SQ_Background`) 0.0))
    (:`BatHit`
      (`AudioComponent.Play` (`self.SQ_BatHit`) 0.0))
    (:`Homerun`
      (`AudioComponent.Play` (`self.SQ_Homerun`) 0.0))
    (:`HomerunSong`
      (`AudioComponent.Play` (`self.SQ_HomerunSong`) 0.0))))

(event `GameOver`
  (bind _defaulttextcolor (`self.DefaultTextColor`))
  ; Game & Player State
  ;; GameOver
  (bind _asbp_wngame_state_base (cast `/Game/Bluprints/Core/BP_WNGameStateBase` (`GameplayStatics.GetGameState`)))
  (`/Game/Bluprints/Core/BP_WNGameStateBase.GameOver` _asbp_wngame_state_base)
  (bind _outactors (`GameplayStatics.GetAllActorsOfClass` "/Game/Bluprints/Core/BP_WNController.BP_WNController_C"))
  (for _array_element _outactors
    (if (`Controller.IsLocalController` _array_element)
      (`/Game/Bluprints/Core/BP_WNController.GotBroadcast` _array_element "Start a new game by entering '!play' \n" _defaulttextcolor)
      (else
        (`/Game/Bluprints/Core/BP_WNController.GotBroadcast` _array_element " \nPlease wait for the host to start a new game." _defaulttextcolor)))
    (bind _asbp_wngame_state_base_2 (cast `/Game/Bluprints/Core/BP_WNGameStateBase` (`GameplayStatics.GetGameState`)))
    (for (_ _array_index) (`/Game/Bluprints/Core/BP_WNGameStateBase.PlayerList` _asbp_wngame_state_base_2)
      (`self.ChangeScoreColorOnTurn` _array_index (`self.DefaultTextColor`)))))

(event `GameStart`
  ; Game & Player State
  ;; GameStart
  (bind _asbp_wngame_state_base (cast `/Game/Bluprints/Core/BP_WNGameStateBase` (`GameplayStatics.GetGameState`)))
  (`/Game/Bluprints/Core/BP_WNGameStateBase.GameStart` _asbp_wngame_state_base))

(event `StopSound`
  (params (SoundName :type String))
  ; Sounds
  ;; StopSound
  (switch `string` SoundName
    (:`Crowd`
      (`AudioComponent.Stop` (`self.SQ_Crowd`)))
    (:`Opening`
      (`AudioComponent.Stop` (`self.SQ_Opening`) :!label _label))
    (:`Background`
      (`AudioComponent.Stop` (`self.SQ_Background`) :!label _label_2))
    (:`BatHit`
      (`AudioComponent.Stop` (`self.SQ_BatHit`) :!label _label_3))
    (:`Homerun`
      (`AudioComponent.Stop` (`self.SQ_Homerun`) :!label _label_4))
    (:`HomerunSong`
      (`AudioComponent.Stop` (`self.SQ_HomerunSong`) :!label _label_5))
    (:`AllSound`
      (`|ExecutionSequence`
        (:`then_0`
          (goto _label))
        (:`then_1`
          (goto _label_2))
        (:`then_2`
          (goto _label_3))
        (:`then_3`
          (goto _label_4))
        (:`then_4`
          (goto _label_5))))))

(event `GameIsReady`
  (params (PlayerController :type "/Game/Bluprints/Core/BP_WNController Object Reference"))
  ; Game & Player State
  ;; Game is Ready
  (`self.WelcomMassage` PlayerController))

(event `SendIDToState`
  (params (ID :type String) (PlayerController :type "/Game/Bluprints/Core/BP_WNController Object Reference"))
  ; Game & Player State
  ;; Set ID
  (bind _asbp_wnplayer_state (cast `/Game/Bluprints/Core/BP_WNPlayerState` (`Controller.PlayerState` PlayerController)))
  (`/Game/Bluprints/Core/BP_WNPlayerState.SetID` _asbp_wnplayer_state ID))

(event `OutDecision`
  (params (PlayerContoroller :type "/Game/Bluprints/Core/BP_WNController Object Reference"))
  ; Game & Player State
  ;; Out Decision
  (bind _asbp_wnplayer_state (cast `/Game/Bluprints/Core/BP_WNPlayerState` (`Controller.PlayerState` PlayerContoroller)))
  (if (<= (`WNPlayerState.RemainingTurn` _asbp_wnplayer_state) 0)
    (`/Game/Bluprints/Core/BP_WNPlayerState.PlayerIsOut` _asbp_wnplayer_state)
    (`self.SendBroadcast` (`KismetStringLibrary.Concat_StrStr` (`WNPlayerState.UserID` _asbp_wnplayer_state) " is out.") (`self.DefaultTextColor`))
    (`self.SetTurn`)
    (else
      (`self.SetTurn`))))

(event `TicketToUser`
  ; Game & Player State
  ;; Give Ticket To User
  (bind _asbp_wngame_state_base (cast `/Game/Bluprints/Core/BP_WNGameStateBase` (`GameplayStatics.GetGameState`)))
  (for _array_element (`/Game/Bluprints/Core/BP_WNGameStateBase.PlayerList` _asbp_wngame_state_base)
    (bind _asbp_wnplayer_state (cast `/Game/Bluprints/Core/BP_WNPlayerState` (`Controller.PlayerState` _array_element)))
    (`WNPlayerState.GiveTicketToUser` _asbp_wnplayer_state)))

(event `SetTurn`
  ; Managing Turn & Time
  ;; Set Turn
  (`self.StopTimer`)
  (bind _isallout (`self.CheckPlayersOutState`))
  (if _isallout
    (`self.GameOver`)
    (`self.SendBroadcast` " \nAll Players Out. Game Over." (struct :`R` 0.5 :`G` 0.066667 :`A` 1.0))
    (`self.GameOver`)
    (else
      (bind _asbp_wngame_state_base (cast `/Game/Bluprints/Core/BP_WNGameStateBase` (`GameplayStatics.GetGameState`)))
      (bind _asbp_wnplayer_state (cast `/Game/Bluprints/Core/BP_WNPlayerState` (`Controller.PlayerState` (`self.CurrentPlayerController`))))
      (if (`WNPlayerState.bIsOut` _asbp_wnplayer_state)
        (bind _turnindex (`/Game/Bluprints/Core/BP_WNGameStateBase.TurnIndex` _asbp_wngame_state_base))
        (`self.ChangeScoreColorOnTurn` _turnindex (struct :`R` 0.338542 :`G` 0.338542 :`B` 0.338542 :`A` 1.0))
        (else
          (`self.ChangeScoreColorOnTurn` _turnindex (`self.DefaultTextColor`))))
      (bind _result (`/Engine/EditorBlueprintResources/StandardMacros.IncrementInt` _turnindex)
        (:`  `
          (bind _playerlist (`/Game/Bluprints/Core/BP_WNGameStateBase.PlayerList` _asbp_wngame_state_base))
          (`/Game/Bluprints/Core/BP_WNGameStateBase.SetTurnIndex` _asbp_wngame_state_base (mod _result (`KismetArrayLibrary.Array_Length` _playerlist)))
          (bind _turnindex_2 (`/Game/Bluprints/Core/BP_WNGameStateBase.TurnIndex` _asbp_wngame_state_base))
          (bind _asbp_wnplayer_state_2 (cast `/Game/Bluprints/Core/BP_WNPlayerState` (`Controller.PlayerState` (`|GetArrayItem` _playerlist _turnindex_2))))
          (if (`WNPlayerState.bIsOut` _asbp_wnplayer_state_2)
            (`self.SetTurn`)
            (else
              (`self.SendBroadcast` (`KismetStringLibrary.Concat_StrStr` (`WNPlayerState.UserID` _asbp_wnplayer_state_2) "'s turn") (struct :`R` 1.0 :`G` 0.502887 :`A` 1.0))
              (`self.ChangeScoreColorOnTurn` _turnindex_2 (`self.ScoreColorOnTurn`))
              (`self.StartTimer`))))))))

(event `BroadcastRemainingTurn`
  ; Managing Turn & Time
  ;; Broadcast Updated Turn
  (bind _asbp_wngame_state_base (cast `/Game/Bluprints/Core/BP_WNGameStateBase` (`GameplayStatics.GetGameState`)))
  (bind _asbp_wnplayer_state (cast `/Game/Bluprints/Core/BP_WNPlayerState` (`Controller.PlayerState` (`|GetArrayItem` (`/Game/Bluprints/Core/BP_WNGameStateBase.PlayerList` _asbp_wngame_state_base) (`/Game/Bluprints/Core/BP_WNGameStateBase.TurnIndex` _asbp_wngame_state_base)))))
  (`self.SendBroadcast` (`KismetStringLibrary.Concat_StrStr` (`WNPlayerState.UserID` _asbp_wnplayer_state) " has " (`KismetStringLibrary.Conv_IntToString` (`WNPlayerState.GetRemainingTurn` _asbp_wnplayer_state)) " chances left.") (`self.DefaultTextColor`)))

(event `SpendTurnbyTimer`
  ; Managing Turn & Time
  ;; Spend Turn by Timer
  (bind _asbp_wngame_state_base (cast `/Game/Bluprints/Core/BP_WNGameStateBase` (`GameplayStatics.GetGameState`)))
  (bind _asbp_wnplayer_state (cast `/Game/Bluprints/Core/BP_WNPlayerState` (`Controller.PlayerState` (`|GetArrayItem` (`/Game/Bluprints/Core/BP_WNGameStateBase.PlayerList` _asbp_wngame_state_base) (`/Game/Bluprints/Core/BP_WNGameStateBase.TurnIndex` _asbp_wngame_state_base)))))
  (`/Game/Bluprints/Core/BP_WNPlayerState.SpendTurn` _asbp_wnplayer_state)
  (`self.SendBroadcast` "Timeout! Turn is over." (struct :`R` 0.75 :`A` 1.0))
  (`self.BroadcastRemainingTurn`)
  (`self.SetTurn`))

(event `StartTimer`
  ; Managing Turn & Time
  ;; Start Timer
  (bind _asbp_wngame_state_base (cast `/Game/Bluprints/Core/BP_WNGameStateBase` (`GameplayStatics.GetGameState`)))
  (bind _returnvalue (`KismetSystemLibrary.K2_SetTimerDelegate` (`|CreateDelegate` :!event `SpendTurnbyTimer`) (`/Game/Bluprints/Core/BP_WNGameStateBase.TurnTime` _asbp_wngame_state_base)))
  (set `self.TurnTimer` _returnvalue)
  (bind _returnvalue_2 (`KismetSystemLibrary.K2_SetTimerDelegate` (`|CreateDelegate` :!event `SendRemainingTime`) 0.1 true))
  (set `self.SendTimeTimer` _returnvalue_2))

(event `StopTimer`
  ; Managing Turn & Time
  ;; Clear Timer
  (`KismetSystemLibrary.K2_ClearAndInvalidateTimerHandle` (`self.TurnTimer`))
  (`KismetSystemLibrary.K2_ClearAndInvalidateTimerHandle` (`self.SendTimeTimer`)))

(event `SendRemainingTime`
  ; Managing Turn & Time
  ;; Send Remaining Time of Turn Timer To Time UI
  (bind _outactors (`GameplayStatics.GetAllActorsOfClass` "/Game/Bluprints/Core/BP_WNController.BP_WNController_C"))
  (for _array_element _outactors
    (`/Game/Bluprints/Core/BP_WNController.SendRemainingTimeToUI` _array_element (`KismetSystemLibrary.K2_GetTimerRemainingTimeHandle` (`self.TurnTimer`)))))

(event `ChangeScoreColorOnTurn`
  (params (PlayerIndex :type Integer) (TextColor :type "LinearColor Structure"))
  ; Managing Turn & Time
  ;; Change Scoreboard Color On Turn
  (bind _outactors (`GameplayStatics.GetAllActorsOfClass` "/Game/Bluprints/Core/BP_WNController.BP_WNController_C"))
  (for _array_element _outactors
    (`/Game/Bluprints/Core/BP_WNController.ChangeScoreTextColor` _array_element PlayerIndex TextColor)))

(fn `CheckPlayersOutState`
  (returns (IsAllOut :type Boolean))
  (bind _asbp_wngame_state_base (cast `/Game/Bluprints/Core/BP_WNGameStateBase` (`GameplayStatics.GetGameState`)))
  (for _array_element (`/Game/Bluprints/Core/BP_WNGameStateBase.PlayerList` _asbp_wngame_state_base)
    (bind _asbp_wnplayer_state (cast `/Game/Bluprints/Core/BP_WNPlayerState` (`Controller.PlayerState` _array_element)))
    (if (not (`WNPlayerState.bIsOut` _asbp_wnplayer_state))
      (return false)))
  (return true))

(fn `UserConstructionScript`)