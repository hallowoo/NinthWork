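; Game state for a turn-based, host-started multiplayer game with a random goal number built from Make3RandNum.
; Player registration lists each controller and sends welcome messages through the game mode, marking joiners out mid-game and giving the local controller the '!play' prompt.
; It also stores the in-play flag, turn index and chat history.
; Resetting zeroes the turn and regenerates the goal number only with authority.
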(event `PlayerRegistration`
  (params (PlayerController :type "/Game/Bluprints/Core/BP_WNController Object Reference"))
  ; Player Registration
  (`KismetArrayLibrary.Array_Add` (`self.PlayerList`) PlayerController)
  (bind _asbp_wnplayer_state (cast `/Game/Bluprints/Core/BP_WNPlayerState` (`Controller.PlayerState` PlayerController)))
  (bind _asbp_wngame_mode_base (cast `/Game/Bluprints/Core/BP_WNGameModeBase` (`GameplayStatics.GetGameMode`)))
  (`/Game/Bluprints/Core/BP_WNGameModeBase.PlayerGetSystemMassage` _asbp_wngame_mode_base (`KismetStringLibrary.Concat_StrStr` " \n" (`WNPlayerState.UserID` _asbp_wnplayer_state) "! Welcome!") PlayerController)
  (bind _asbp_wngame_state_base (cast `/Game/Bluprints/Core/BP_WNGameStateBase` (`GameplayStatics.GetGameState`)))
  (if (`/Game/Bluprints/Core/BP_WNGameStateBase.IsGameInPlay` _asbp_wngame_state_base)
    (`/Game/Bluprints/Core/BP_WNGameModeBase.PlayerGetSystemMassage` _asbp_wngame_mode_base "Please wait until the game ends. \n" PlayerController)
    (`WNPlayerState.PlayerOut` _asbp_wnplayer_state)
    (elif (`Controller.IsLocalController` PlayerController)
      (`/Game/Bluprints/Core/BP_WNGameModeBase.PlayerGetSystemMassage` _asbp_wngame_mode_base "To start a game, enter '!play' \n" PlayerController)
      (else
        (`/Game/Bluprints/Core/BP_WNGameModeBase.PlayerGetSystemMassage` _asbp_wngame_mode_base "Please wait until the host starts the game. \n" PlayerController)))))

(event `MakeGoalNumber`
  ; Set Goal Number
  (bind _returnvalue (`Make3RandNum.Make3RandNum`))
  (`self.SetGoalNumber` _returnvalue))

(event `GameStart`
  ; GameStart
  (set `self.IsGameInPlay` true))

(event `GameOver`
  ; GameOver
  (set `self.IsGameInPlay` false))

(event `ResetGameState`
  ; Reset Game
  (set `self.TurnIndex` 0)
  (if (`self.HasAuthority`)
    (`self.MakeGoalNumber`)))

(event `SetTurnIndex`
  (params (TurnIndex :type Integer))
  ; Set Current Turn Index
  (set `self.TurnIndex` TurnIndex))

(event `SaveChatList`
  (params (Massage :type String))
  ; SaveChat
  (`KismetArrayLibrary.Array_Add` (`self.ChatMassage`) Massage))

(fn `GetTurnIndex`
  (returns (CurrentTurnIndex :type Integer))
  (return (`self.TurnIndex`)))

(fn `UserConstructionScript`)